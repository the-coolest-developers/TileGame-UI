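; Player controller for a top-down building game that drives the MainPawn camera and feeds cursor input to construction placement.
; On BeginPlay it spawns the construction manager and tile ghost, then creates the HUD with references to itself and the ghost.
; Axis input and screen-edge mouse checks pan the pawn, with key speed scaled by zoom, which adjusts two spring arms.
; In build mode, Tick updates the ghost's cursor world position and Deselect kills it.
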(event `self.ReceiveBeginPlay`
  (bind _returnvalue (`KismetMathLibrary.MakeTransform` (0.0 0.0 0.0)))
  ;[1 1 1] BeginPlay
  (`|ExecutionSequence`
    (:`then_0`
      (`self.ReferenceCast`))
    (:`then_1`
      (bind _returnvalue_2 (`|SpawnActorFromClass` "/Game/Blueprints/Tile_BP/Construction/ConstructionManager_BP.ConstructionManager_BP_C" _returnvalue "AlwaysSpawn" "OverrideRootScale" null null))
      (set `self.ConstructionManagerRef` _returnvalue_2))
    (:`then_2`
      (bind _returnvalue_3 (`|SpawnActorFromClass` "/Game/Blueprints/Tile_BP/TileGhost_BP.TileGhost_BP_C" _returnvalue "AlwaysSpawn" "OverrideRootScale" null self null))
      (set `self.GhostTileRef` _returnvalue_3))
    (:`then_3`
      (`WidgetBlueprintLibrary.SetInputMode_GameAndUIEx` self null "LockAlways" false)
      (`self.CreateHuds`)
      (`UserWidget.AddToViewport` (`self.HUDRef`) 0))))

(event `self.ReceiveTick`
  (params (DeltaSeconds :type "Float (single-precision)"))
  (bind _returnvalue (`self.GetTransform` (`self.MainPawnReferenceVariable`)))
  ;[1 1 1] MoveByMouse
  (bind (_forward _back _left _right) (`self.CheckMouseDirections`))
  (`self.K2_SetActorTransform` (`self.MainPawnReferenceVariable`) (`KismetMathLibrary.MakeTransform` (+ (`KismetMathLibrary.TransformDirection` _returnvalue (+ (* (100.0 0.0 0.0) _forward) (* (-100.0 0.0 0.0) _back) (* (0.0 -100.0 0.0) _left) (* (0.0 100.0 0.0) _right))) (.location _returnvalue)) (.rotation _returnvalue) (.scale _returnvalue)) false false)
  (if (`self.BuildModeState`)
    (if (!= (`self.GhostTileRef`) null)
      (set `/Game/Blueprints/Tile_BP/TileGhost_BP.CursorWorldPosition` (`/Game/Blueprints/Libraries/FunctionLibrary.Set Cursor World Position` self (`self.SetSightDistance`)) (`self.GhostTileRef`)))))

(event `InputAction|Deselect`
  (params (Key :type "Key Structure"))
  (:`Pressed`
    (if (`self.BuildModeState`)
      (`/Game/Blueprints/Tile_BP/TileGhost_BP.KillGhost` (`self.GhostTileRef`))
      (set `self.BuildModeState` false))))

(event `InputAxis|InputAxisMoveX`
  (params (AxisValue :type "Float (single-precision)"))
  ;[1 1 1] MoveByButtons
  ;;[1 1 1] MovementAxisXByButtons
  (if (not (`self.DisableCameraNavigation`))
    (`self.K2_SetActorTransform` (`self.MainPawnReferenceVariable`) (`self.MovementX` AxisValue (`self.MovementSpeedCalculation`) (`self.FastMoveMultiplier`) (`self.MainPawnReferenceVariable`)) false false)))

(event `InputAction|ZoomIn`
  (params (Key :type "Key Structure"))
  ;[1 1 1] Zoom
  ;;[1 1 1] ZoomIn
  (:`Pressed`
    ;;;[1 1 1] ZoomInCamera1
    (set `SpringArmComponent.TargetArmLength` (`KismetMathLibrary.FClamp` (- (`SpringArmComponent.TargetArmLength` (`/Game/Blueprints/Player/MainPawn.SpringArm 1` (`self.MainPawnReferenceVariable`))) (`self.ZoomSensitivity`)) 500.0 (`self.MaxArm(Zoom)Distanse`)) (`/Game/Blueprints/Player/MainPawn.SpringArm 1` (`self.MainPawnReferenceVariable`)))
    ;;;[1 1 1] ZoomInCamera2
    (set `SpringArmComponent.TargetArmLength` (`KismetMathLibrary.FClamp` (- (`SpringArmComponent.TargetArmLength` (`/Game/Blueprints/Player/MainPawn.SpringArm 2` (`self.MainPawnReferenceVariable`))) (`self.ZoomSensitivity`)) 500.0 (`self.MaxArm(Zoom)Distanse`)) (`/Game/Blueprints/Player/MainPawn.SpringArm 2` (`self.MainPawnReferenceVariable`)))))

(event `InputAxis|InputAxisMoveY`
  (params (AxisValue :type "Float (single-precision)"))
  ;[1 1 1] MoveByButtons
  ;;[1 1 1] MovementAxisYByButtons
  (if (not (`self.DisableCameraNavigation`))
    (`self.K2_SetActorTransform` (`self.MainPawnReferenceVariable`) (`self.MovementY` AxisValue (`self.MovementSpeedCalculation`) (`self.FastMoveMultiplier`) (`self.MainPawnReferenceVariable`)) false false)))

(event `InputAction|ZoomOut`
  (params (Key :type "Key Structure"))
  ;[1 1 1] Zoom
  ;;[1 1 1] ZoomOut
  (:`Pressed`
    ;;;[1 1 1] ZoomOutCamera1
    (set `SpringArmComponent.TargetArmLength` (`KismetMathLibrary.FClamp` (+ (`SpringArmComponent.TargetArmLength` (`/Game/Blueprints/Player/MainPawn.SpringArm 1` (`self.MainPawnReferenceVariable`))) (`self.ZoomSensitivity`)) 500.0 (`self.MaxArm(Zoom)Distanse`)) (`/Game/Blueprints/Player/MainPawn.SpringArm 1` (`self.MainPawnReferenceVariable`)))
    ;;;[1 1 1] ZoomOutCamera2
    (set `SpringArmComponent.TargetArmLength` (`KismetMathLibrary.FClamp` (+ (`SpringArmComponent.TargetArmLength` (`/Game/Blueprints/Player/MainPawn.SpringArm 2` (`self.MainPawnReferenceVariable`))) (`self.ZoomSensitivity`)) 500.0 (`self.MaxArm(Zoom)Distanse`)) (`/Game/Blueprints/Player/MainPawn.SpringArm 2` (`self.MainPawnReferenceVariable`)))))

(event `InputAction|ZoomReset`
  (params (Key :type "Key Structure"))
  ;[1 1 1] Zoom
  ;;[1 1 1] ResetZoom
  (:`Pressed`
    ;;;[1 1 1] ResetZoomCamera1
    (set `SpringArmComponent.TargetArmLength` 1000.0 (`/Game/Blueprints/Player/MainPawn.SpringArm 1` (`self.MainPawnReferenceVariable`)))
    ;;;[1 1 1] ResetZoomCamera2
    (set `SpringArmComponent.TargetArmLength` 1000.0 (`/Game/Blueprints/Player/MainPawn.SpringArm 2` (`self.MainPawnReferenceVariable`)))))

(fn `CheckMouseBackDirection_0`
  (returns (NewParam :type "Float (double-precision)"))
  (bind (_returnvalue_x _returnvalue_y) (`KismetMathLibrary.BreakVector2D` (`WidgetLayoutLibrary.GetViewportSize`)))
  ;[1 1 1] Back
  (bind _returnvalue (`WidgetLayoutLibrary.GetMousePositionOnViewport`))
  (return (- (`KismetMathLibrary.FClamp` (`KismetMathLibrary.NormalizeToRange` (`.Y` (`KismetMathLibrary.BreakVector2D` _returnvalue)) (* _returnvalue_y 1.5) _returnvalue_y) 0.9) 0.9)))

(fn `CheckMouseDirections`
  (returns (Forward :type "Float (double-precision)") (Back :type "Float (double-precision)") (Left :type "Float (double-precision)") (Right :type "Float (double-precision)"))
  (bind _newparam (`self.CheckMouseRightDirection`))
  (bind _newparam_2 (`self.CheckMouseLeftDirection`))
  (bind _newparam_3 (`self.CheckMouseBackDirection_0`))
  (bind _newparam_4 (`self.CheckMouseForwardDirection`))
  (return _newparam_4 _newparam_3 _newparam_2 _newparam))

(fn `CheckMouseForwardDirection`
  (returns (NewParam :type "Float (double-precision)"))
  (bind _returnvalue_x (`KismetMathLibrary.BreakVector2D` (`WidgetLayoutLibrary.GetViewportSize`)))
  ;[1 1 1] Forward
  (bind _returnvalue (`WidgetLayoutLibrary.GetMousePositionOnViewport`))
  (return (- 1.0 (`KismetMathLibrary.FClamp` (`KismetMathLibrary.NormalizeToRange` (`.Y` (`KismetMathLibrary.BreakVector2D` _returnvalue)) 0.0 (* _returnvalue_x 0.05)) 0.9))))

(fn `CheckMouseLeftDirection`
  (returns (NewParam :type "Float (double-precision)"))
  (bind _returnvalue_x (`KismetMathLibrary.BreakVector2D` (`WidgetLayoutLibrary.GetViewportSize`)))
  ;[1 1 1] Left
  (bind _returnvalue (`WidgetLayoutLibrary.GetMousePositionOnViewport`))
  (return (- 1.0 (`KismetMathLibrary.FClamp` (`KismetMathLibrary.NormalizeToRange` (`KismetMathLibrary.BreakVector2D` _returnvalue) 0.0 (* _returnvalue_x 0.05)) 0.9))))

(fn `CheckMouseRightDirection`
  (returns (NewParam :type "Float (double-precision)"))
  (bind (_returnvalue_x _returnvalue_y) (`KismetMathLibrary.BreakVector2D` (`WidgetLayoutLibrary.GetViewportSize`)))
  ;[1 1 1] Right
  (bind _returnvalue (`WidgetLayoutLibrary.GetMousePositionOnViewport`))
  (return (- (`KismetMathLibrary.FClamp` (`KismetMathLibrary.NormalizeToRange` (`KismetMathLibrary.BreakVector2D` _returnvalue) (* _returnvalue_x 1.65) _returnvalue_y) 0.9) 0.9)))

(fn `MovementSpeedCalculation`
  (returns (MoveSensetivity :type "Float (double-precision)"))
  (return (`KismetMathLibrary.FClamp` (/ (`SpringArmComponent.TargetArmLength` (`/Game/Blueprints/Player/MainPawn.SpringArm 1` (`self.MainPawnReferenceVariable`))) 100.0) 5.0 20.0)))

(fn `SetSightDistance`
  (returns (SightDistance :type "Float (double-precision)"))
  (return (+ (`self.SightDistance`) (`SpringArmComponent.TargetArmLength` (`/Game/Blueprints/Player/MainPawn.SpringArm 1` (`self.MainPawnReferenceVariable`))))))

(fn `UserConstructionScript`)