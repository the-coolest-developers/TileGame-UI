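; Placement preview actor for tile building that shows the selected tile's mesh snapped to a grid at the cursor position.
; TileBuild briefly spawns the tile class to read its mesh and construction proxy, restarts the ghost with them, then destroys it.
; Spawning and killing the ghost toggle the controller's build mode and a Tick gate that drives snapped movement.
; GetTileStructure packages the class, proxy, transform and mesh.
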(event `OnSpawn`
  (params (DisplayMesh :type "StaticMesh Object Reference") (TileClass :type "/Game/Blueprints/Tile_BP/TileMaster_BP Class Reference") (ConstructionProxy :type "/Game/Blueprints/Tile_BP/Construction/ConstructionProxy_BP Class Reference"))
  ;[1 1 1] SpawnGhost
  (if (not (`self.IsActive`))
    (set `self.TileClass` TileClass)
    (set `self.ConstructionProxy` ConstructionProxy)
    (set `self.DisplayMesh` DisplayMesh)
    (set `self.IsActive` true)
    (set `/Game/Blueprints/Player/MainPawnController.BuildModeState` true (`self.ControllerRef`))
    (`StaticMeshComponent.SetStaticMesh` (`self.GhostTileMesh`) (`self.DisplayMesh`))
    (`self.OpenTickGate`)))

(event `KillGhost`
  ;[1 1 1] KillGhost
  (set `self.TileClass` null)
  (set `self.ConstructionProxy` null)
  (`self.CloseTickGate`)
  (set `self.DisplayMesh` null)
  (set `self.IsActive` false)
  (set `/Game/Blueprints/Player/MainPawnController.BuildModeState` false (`self.ControllerRef`))
  (`StaticMeshComponent.SetStaticMesh` (`self.GhostTileMesh`) (`self.DisplayMesh`)))

(event `/Game/Blueprints/Interfaces/I_HUD.TileBuild`
  (params (MainTile :type "/Game/Blueprints/Tile_BP/TileMaster_BP Class Reference"))
  ;[1 1 1] TileBuild
  (bind _returnvalue (`|SpawnActorFromClass` MainTile (`KismetMathLibrary.MakeTransform` (0.0 0.0 0.0)) "Undefined" "OverrideRootScale" null (`self.ControllerRef`) null))
  (`|ExecutionSequence`
    (:`then_0`
      (bind _astile_master_bp (castclass `/Game/Blueprints/Tile_BP/TileMaster_BP` MainTile))
      (`self.KillGhost`)
      (`self.OnSpawn` (`/Game/Blueprints/Tile_BP/TileMaster_BP.DisplayMesh` _returnvalue) _astile_master_bp (`/Game/Blueprints/Tile_BP/TileMaster_BP.ConstructionProxy` _returnvalue)))
    (:`then_1`
      (`self.K2_DestroyActor` _returnvalue))))

(event `self.ReceiveTick`
  (params (DeltaSeconds :type "Float (single-precision)"))
  ;[1 1 1] Tick
  (`/Engine/EditorBlueprintResources/StandardMacros.Gate` true :!label _label
    (:`Exit`
      (`self.K2_SetActorLocation` self (`self.SetGridSnapVector`) false false))))

(event `OpenTickGate`
  ;[1 1 1] Tick
  (goto _label :!via `Open`))

(event `CloseTickGate`
  ;[1 1 1] Tick
  (goto _label :!via `Close`))

(fn `GetTileStructure`
  (returns (Structure :type "/Game/Blueprints/Structs/Tile_Structure Structure"))
  (return (make `/Game/Blueprints/Structs/Tile_Structure` (`self.TileClass`) (`self.ConstructionProxy`) (`KismetMathLibrary.MakeTransform` (`self.K2_GetActorLocation`) (`self.K2_GetActorRotation`)) (`self.DisplayMesh`))))

(fn `SetCursorPosition`
  (params (CursorLocation :type "Vector Structure"))
  (set `self.CursorWorldPosition` CursorLocation)
  (return))

(fn `SetGridSnapVector`
  (returns (GridSnap :type "Vector Structure"))
  (bind (_cursorworldposition_x _cursorworldposition_y _cursorworldposition_z) (`KismetMathLibrary.BreakVector` (`self.CursorWorldPosition`)))
  (bind _gridsize (`self.GridSize`))
  (return (`KismetMathLibrary.MakeVector` (`/Game/Blueprints/Libraries/FunctionLibrary.GridSnap` _cursorworldposition_x _gridsize) (`/Game/Blueprints/Libraries/FunctionLibrary.GridSnap` _cursorworldposition_y _gridsize) (`/Game/Blueprints/Libraries/FunctionLibrary.GridSnap` _cursorworldposition_z _gridsize))))

(fn `UserConstructionScript`)