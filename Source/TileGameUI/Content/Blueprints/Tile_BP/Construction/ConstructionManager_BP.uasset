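; Construction manager actor that queues tile builds, using proxy actors as stand-ins for the final tiles.
; QueueTile spawns a proxy with a display mesh, calls TileCompleted on it immediately, then records proxy and config in parallel arrays.
; FinishTile reads the config one past the proxy's index, removes that index's entries, spawns the tile and destroys the proxy.
; BindTileCompleted binds to a proxy's built event but is not called here.
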(event `BindTileCompleted`
  (params (Proxy :type "/Game/Blueprints/Tile_BP/Construction/ConstructionProxy_BP Object Reference"))
  (add `/Game/Blueprints/Tile_BP/Construction/ConstructionProxy_BP.TileBuilded` Proxy (`|CreateDelegate` :!event `TileCompleted`)))

(event `TileCompleted`
  (params (Proxy :type "/Game/Blueprints/Tile_BP/Construction/ConstructionProxy_BP Object Reference"))
  (`self.FinishTile` Proxy))

(fn `FinishTile`
  (params (Proxy :type "/Game/Blueprints/Tile_BP/Construction/ConstructionProxy_BP Object Reference"))
  (locals (Index :type Integer) (Confug :type "/Game/Blueprints/Structs/Tile_Structure Structure"))
  (bind _queue (`self.Queue`))
  (bind _index (`local.Index`))
  (bind _proxies (`self.Proxies`))
  (bind _output_get (set `local.Index` (`KismetArrayLibrary.Array_Find` _proxies Proxy)))
  (bind _output_get_2 (set `local.Confug` (`|GetArrayItem` _queue (+ _output_get 1))))
  (`KismetArrayLibrary.Array_Remove` _queue _index)
  (`KismetArrayLibrary.Array_Remove` _proxies _index)
  (bind (_tileclass _proxyclass _transform) (break `/Game/Blueprints/Structs/Tile_Structure` _output_get_2))
  (`|SpawnActorFromClass` _tileclass _transform "Undefined" "OverrideRootScale" null null null)
  (`self.K2_DestroyActor` Proxy))

(fn `Queue Tile`
  (params (NewParam :type "/Game/Blueprints/Structs/Tile_Structure Structure"))
  (bind (_tileclass _proxyclass _transform _displaymesh) (break `/Game/Blueprints/Structs/Tile_Structure` NewParam))
  (bind _returnvalue (`|SpawnActorFromClass` _proxyclass _transform "AlwaysSpawn" "OverrideRootScale" null _displaymesh null))
  (`self.TileCompleted` _returnvalue)
  (`KismetArrayLibrary.Array_Add` (`self.Proxies`) _returnvalue)
  (`KismetArrayLibrary.Array_Add` (`self.Queue`) NewParam))

(fn `UserConstructionScript`)